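; Gameplay game mode that starts the level's music and puts the player into a randomly chosen color character.
; On BeginPlay it spawns a red, green or blue character at the PlayerStart with roughly equal odds, then has the player controller possess it.
; It first loads the SaveAudio save slot, if present, to apply camera sensitivity to GameplayPC and push the three saved colors into the MPC_GameColors material parameter collection.
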(event Custom|LoadSaveColors
  (bind _returnvalue (SaveGame|DoesSaveGameExist "SaveAudio"))
  (if _returnvalue
    (bind _returnvalue_2 (SaveGame|LoadGamefromSlot "SaveAudio"))
    (bind _assave_audio (Utilities|Casting|CastToSaveAudio _returnvalue_2))
    (bind _asgameplay_pc (Utilities|Casting|CastToGameplayPC (Game|GetPlayerController 0)))
    (Class|GameplayPC|SetCameraSensitivity _asgameplay_pc (Variables|/Game/Assets/Audio/SaveAudio.SaveAudio_C|GetSensitivity _assave_audio))
    (Rendering|Material|SetVectorParameterValue "/Game/Assets/Materials/MPC_GameColors.MPC_GameColors" "RedColor" (Variables|/Game/Assets/Audio/SaveAudio.SaveAudio_C|GetRedColor _assave_audio) :!class /Script/Engine.KismetMaterialLibrary)
    (Rendering|Material|SetVectorParameterValue "/Game/Assets/Materials/MPC_GameColors.MPC_GameColors" "GreenColor" (Variables|/Game/Assets/Audio/SaveAudio.SaveAudio_C|GetGreenColor _assave_audio) :!class /Script/Engine.KismetMaterialLibrary)
    (Rendering|Material|SetVectorParameterValue "/Game/Assets/Materials/MPC_GameColors.MPC_GameColors" "BlueColor" (Variables|/Game/Assets/Audio/SaveAudio.SaveAudio_C|GetBlueColor _assave_audio) :!class /Script/Engine.KismetMaterialLibrary)))

(event EventBeginPlay
  (CallFunction|LoadSaveColors)
  (Audio|PlaySound2D "/Game/Assets/Audio/Song/MS_BigModeSong.MS_BigModeSong" 1.0 1.0 0.0 0 0)
  (bind _returnvalue (Actor|GetActorOfClass "/Script/Engine.PlayerStart"))
  (bind _output_get (Variables|Default|SetRandomSpawnCharacterValue (Math|Random|RandomFloat)))
  (if (<= _output_get 0.33)
    (bind _returnvalue_2 (Game|SpawnActorfromClass "/Game/Blueprints/Characters/BP_RedCharacter.BP_RedCharacter_C" (Math|Transform|MakeTransform (Transformation|GetActorLocation _returnvalue) (Transformation|GetActorRotation _returnvalue) "1.000000,1.000000,1.000000") "Undefined" "MultiplyWithRoot" 0 0))
    (Variables|Default|SetSpawnedCharacter _returnvalue_2)
    (elif (<= _output_get 0.66)
      (bind _returnvalue_3 (Game|SpawnActorfromClass "/Game/Blueprints/Characters/BP_GreenCharacter.BP_GreenCharacter_C" (Math|Transform|MakeTransform (Transformation|GetActorLocation _returnvalue) (Transformation|GetActorRotation _returnvalue) "1.000000,1.000000,1.000000") "Undefined" "MultiplyWithRoot" 0 0))
      (Variables|Default|SetSpawnedCharacter _returnvalue_3)
      (else
        (bind _returnvalue_4 (Game|SpawnActorfromClass "/Game/Blueprints/Characters/BP_BlueCharacter.BP_BlueCharacter_C" (Math|Transform|MakeTransform (Transformation|GetActorLocation _returnvalue) (Transformation|GetActorRotation _returnvalue) "1.000000,1.000000,1.000000") "Undefined" "MultiplyWithRoot" 0 0))
        (Variables|Default|SetSpawnedCharacter _returnvalue_4))))
  (Pawn|Possess (Game|GetPlayerController 0) (Variables|Default|GetSpawnedCharacter)))

(event EventTick
  (params (DeltaSeconds :type Float%20%28single-precision%29)))

(fn ConstructionScript)