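; Gameplay Game State that handles game over and combo audio feedback.
; When health is depleted, it shows the game over menu, switches to UI-only input with the cursor visible, and plays a sound.
; It then loads or creates the SaveAudio save object and writes the score if it beats BestScore.
; Combo increases play one of two random sounds whenever the count is a multiple of ten.
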(event EventBeginPlay)

(event EventTick
  (params (DeltaSeconds :type Float%20%28single-precision%29)))

(event EventOnHealthDepleted
  (bind _returnvalue (Game|GetPlayerController 0))
  (bind _returnvalue_2 (UserInterface|CreateWidget "/Game/Blueprints/UI/BP_GameOverMenu.BP_GameOverMenu_C"))
  (UserInterface|Viewport|AddtoViewport _returnvalue_2 10)
  (Variables|/Script/Engine.PlayerController|SetbShowMouseCursor _returnvalue true)
  (Input|SetInputModeUIOnly _returnvalue 0 "DoNotLock" false)
  (Input|SetIgnoreMoveInput _returnvalue true)
  (Audio|PlaySound2D "/Game/Assets/Audio/Character/slaymode.slaymode" 1.0 1.0 0.0 0 0)
  (bind _returnvalue_3 (SaveGame|DoesSaveGameExist "SaveAudio"))
  (if _returnvalue_3
    (bind _returnvalue_4 (SaveGame|LoadGamefromSlot "SaveAudio"))
    (bind _assave_audio (Utilities|Casting|CastToSaveAudio _returnvalue_4))
    (Variables|Default|SetSaveAudioREF _assave_audio)
    (else
      (bind _returnvalue_5 (SaveGame|CreateSaveGameObject "/Game/Assets/Audio/SaveAudio.SaveAudio_C"))
      (Variables|Default|SetSaveAudioREF _returnvalue_5)))
  (bind _returnvalue_6 (Class|GameplayGS|GetScore))
  (if (> _returnvalue_6 (Variables|/Game/Assets/Audio/SaveAudio.SaveAudio_C|GetBestScore (Variables|Default|GetSaveAudioREF)))
    (Variables|/Game/Assets/Audio/SaveAudio.SaveAudio_C|SetBestScore (Variables|Default|GetSaveAudioREF) _returnvalue_6)
    (SaveGame|SaveGametoSlot (Variables|Default|GetSaveAudioREF) "SaveAudio")))

(event EventOnComboIncreased
  (if (== (Math|Integer|%(Integer) (Variables|Default|GetCurrentComboCount) 10) 0)
    (if (Math|Random|RandomBool)
      (Audio|PlaySound2D "/Game/Assets/Audio/Character/chromacombo1.chromacombo1" 1.0 1.0 0.0 0 0)
      (else
        (Audio|PlaySound2D "/Game/Assets/Audio/Character/chromacombo2.chromacombo2" 1.0 1.0 0.0 0 0)))))

(fn ConstructionScript)