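; Character component that gives the player a right-mouse grapple hook that doubles as body-swapping possession.
; Camera line trace, with sphere-trace fallback, finds and outlines possessable characters; otherwise the grapple fires.
; Tick animates the cable and pulls the character toward hit points until release or timeout.
; Possession flies the character to its target, aligns rotation, switches control, destroys the old body and awards score and health.
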(event Custom|StopGrapple
  (bind _parentcharacter (Variables|Default|GetParentCharacter))
  (bind _charactermovement (Variables|/Script/Engine.Character|GetCharacterMovement _parentcharacter))
  ;[1 1 1] StopGrapple
  (if (Variables|Default|GetIsGrappling)
    (if (Class|NavMovementComponent|IsFlying _charactermovement)
      (Pawn|Components|CharacterMovement|SetMovementMode _charactermovement "MOVE_Falling" 0))
    (Variables|Default|SetGrappleCurrentTime 0.0)
    (Variables|Default|SetIsGrappling false)
    (Variables|Default|SetCanGrapple false)
    (Rendering|SetVisibility (Variables|Default|GetCable) false false)
    (Utilities|FlowControl|Delay (Variables|Default|GetGrappleCooldown))
    (Variables|Default|SetCanGrapple true)))

(event Custom|UpdatePossess
  (params (DeltaSeconds :type Float%20%28double-precision%29))
  (bind _returnvalue (Game|GetPlayerController 0))
  (bind _returnvalue_2 (Components|GetOwner))
  (bind _parentcharacter (Variables|Default|GetParentCharacter))
  (bind _cachedinterptorotation (Variables|Default|GetCachedInterpToRotation))
  (bind _parentcharacter_2 (Variables|Default|GetParentCharacter))
  (bind _parentcharacter_3 (Variables|Default|GetParentCharacter))
  (bind _grapplepoint (Variables|Default|GetGrapplePoint))
  (bind _returnvalue_3 (Transformation|GetActorLocation _parentcharacter_3))
  (bind _returnvalue_4 (Transformation|GetActorLocation _grapplepoint))
  (bind _returnvalue_5 (Pawn|GetControlRotation _parentcharacter_2 :!class /Script/Engine.Pawn))
  (if (Variables|Default|GetIsPossessing)
    (Variables|Default|GetCharacterPossessing
      (:then
        (Variables|/Script/Engine.MovementComponent|SetVelocity (Variables|/Script/Engine.Character|GetCharacterMovement _parentcharacter_3) "0, 0, 0")
        (Transformation|SetActorLocation _parentcharacter_3 (+ _returnvalue_3 (* (Math|Vector|Normalize (- _returnvalue_4 _returnvalue_3)) (* (Variables|Default|GetPossessMoveSpeed) DeltaSeconds))) false false)
        (if (<= (Class|KismetMathLibrary|VectorDistanceSquared _returnvalue_3 _returnvalue_4) 5e+03)
          (Pawn|SetControlRotation (Pawn|GetController _parentcharacter_2) (Math|Interpolation|RInterpTo _returnvalue_5 _cachedinterptorotation DeltaSeconds 6.0))
          (if (Utilities|Operators|EqualEqual _returnvalue_5 _cachedinterptorotation 2e+01)
            (Variables|Default|SetIsPossessing false)
            ;[1 1 1] Complete possession.
            (CallFunction|SetPossessCooldown (Variables|/Game/Blueprints/Characters/BP_BaseCharacter.BP_BaseCharacter_C|GetBP_GrappleComponent (Variables|Default|GetCharacterPossessing)) false (Variables|Default|GetPossessCooldown))
            (Pawn|Possess _returnvalue (Variables|Default|GetCharacterPossessing))
            (Rendering|SetRenderCustomDepth (Variables|/Script/Engine.Character|GetMesh (Variables|Default|GetCharacterPossessing)) false)
            (bind _asbp_base_character (Utilities|Casting|CastToBP_BaseCharacter _returnvalue_2))
            (Rendering|SetRenderCustomDepth (Variables|/Script/Engine.Character|GetMesh _asbp_base_character) false)
            (Actor|DestroyActor _returnvalue_2)
            (Variables|Default|SetCharacterPossessing 0)
            (bind _asgameplay_pc (Utilities|Casting|CastToGameplayPC _returnvalue))
            (Class|GameplayPC|SetCameraRotationEnabled _asgameplay_pc true)
            (bind _asbp_gameplay_gs (Utilities|Casting|CastToBP_GameplayGS (Game|GetGameState)))
            (Class|GameplayGS|AddScore _asbp_gameplay_gs (Variables|Default|GetPointsOnPossess))
            (Class|GameplayGS|IncreaseHealth _asbp_gameplay_gs (Variables|Default|GetHealthOnPossess)))))
      (:else
        ;[1 1 1] The guy being possessed died/became invalid while the player was traveling. Reset current guy.
        (Collision|SetCollisionEnabled (Variables|/Script/Engine.Character|GetCapsuleComponent _parentcharacter) "QueryAndPhysics")
        (Variables|Default|SetIsPossessing false)
        (Variables|Default|SetCharacterPossessing 0)
        (CallFunction|StopGrapple)
        (bind _asgameplay_pc_2 (Utilities|Casting|CastToGameplayPC (Pawn|GetController _parentcharacter)))
        (Class|GameplayPC|SetCameraRotationEnabled _asgameplay_pc_2 true)))))

(event Custom|HighlightPossess
  ;[1 1 1] HighlightPossess
  (bind _asbp_base_character (Utilities|Casting|CastToBP_BaseCharacter (Components|GetOwner)))
  (if (and (Pawn|IsPlayerControlled _asbp_base_character) (Variables|Default|GetCanPossess))
    (bind (_hitres _ifhit) (CallFunction|RayCastforPossession))
    (if _ifhit
      (bind _aspawn (Utilities|Casting|CastToPawn (.HitActor (Collision|BreakHitResult _hitres)))
        (:then
          (Utilities|IsValid (Variables|Default|GetHighlightedCharacter)
            (:Is%20Valid
              (bind _aspawn_2 (Utilities|Casting|CastToPawn (Variables|Default|GetHighlightedCharacter))
                (:then
                  (if (!= _aspawn _aspawn_2)
                    (bind _asbp_base_character_2 (Utilities|Casting|CastToBP_BaseCharacter (Variables|Default|GetHighlightedCharacter)))
                    (Rendering|SetRenderCustomDepth (Variables|/Script/Engine.Character|GetMesh _asbp_base_character_2) false)
                    (bind _output_get (Variables|Default|SetHighlightedCharacter (.HitActor (Collision|BreakHitResult _hitres)) :!label _label))
                    (bind _asbp_base_character_3 (Utilities|Casting|CastToBP_BaseCharacter _output_get))
                    (Rendering|SetRenderCustomDepth (Variables|/Script/Engine.Character|GetMesh _asbp_base_character_3) true)))
                (:CastFailed
                  (goto _label))))
            (:Is%20Not%20Valid
              (goto _label))))
        (:CastFailed
          (Utilities|IsValid (Variables|Default|GetHighlightedCharacter) :!label _label_2
            (:Is%20Valid
              (bind _asbp_base_character_4 (Utilities|Casting|CastToBP_BaseCharacter (Variables|Default|GetHighlightedCharacter)))
              (Rendering|SetRenderCustomDepth (Variables|/Script/Engine.Character|GetMesh _asbp_base_character_4) false)
              (Variables|Default|SetHighlightedCharacter 0)))))
      (else
        (goto _label_2)))))

(event Custom|GrappleMovement
  (bind _parentcharacter (Variables|Default|GetParentCharacter))
  (bind _parentcharacter_2 (Variables|Default|GetParentCharacter))
  (bind _returnvalue (Transformation|GetActorLocation _parentcharacter))
  (bind _charactermovement (Variables|/Script/Engine.Character|GetCharacterMovement _parentcharacter_2))
  ;[1 1 1] GrappleMovement
  (Variables|/Script/Engine.MovementComponent|SetVelocity _charactermovement (+ (Variables|/Script/Engine.MovementComponent|GetVelocity _charactermovement) (* (Math|Vector|GetUnitDirection(Vector) _returnvalue (Transformation|GetActorLocation (Variables|Default|GetGrapplePoint))) (* (Variables|Default|GetGrappleVelocity) (Math|Float|Clamp(Float) (+ (/ (Math|Vector|Distance(Vector) (Variables|Default|GetGrappleStart) _returnvalue) (Variables|Default|GetDist)) 0.5)))))))

(event Custom|DrawGrapple
  (bind _grapplecurrenttime (Variables|Default|GetGrappleCurrentTime))
  (bind _returnvalue (* _grapplecurrenttime 8.0))
  (bind _returnvalue_2 (Math|Float|Clamp(Float) _returnvalue))
  ;[1 1 1] DrawGrapple
  (if (and (== _returnvalue_2 1.0) (not (Variables|Default|GetHasHit)))
    (CallFunction|StopGrapple))
  (Variables|/Script/CableComponent.CableComponent|SetEndLocation (Variables|Default|GetCable) (* (Math|Transform|InverseTransformLocation (Transformation|GetActorTransform (Variables|Default|GetParentCharacter)) (Transformation|GetActorLocation (Variables|Default|GetGrapplePoint))) _returnvalue_2)))

(event Custom|PlayTimerSound
  ;[1 1 1] StartGrapple
  (if (and (Variables|Default|GetIsGrappling) (Variables|Default|GetHasHit))
    (Audio|PlaySound2D "/Engine/VREditor/Sounds/UI/Click_on_Button_Cue.Click_on_Button_Cue" 1.0 1.0 0.0 0 0)))

(event Custom|Possess
  (params (ActorToPossess :type Actor%20Object%20Reference))
  ;[1 1 1] Possesion
  (bind _asbp_base_character (Utilities|Casting|CastToBP_BaseCharacter ActorToPossess))
  (bind _output_get (Variables|Default|SetCharacterPossessing _asbp_base_character))
  (Variables|Default|SetCachedInterpToRotation (Transformation|GetActorRotation _output_get))
  (Variables|Default|SetIsPossessing true)
  (Collision|SetCollisionEnabled (Variables|/Script/Engine.Character|GetCapsuleComponent (Variables|Default|GetParentCharacter)) "NoCollision")
  (bind _returnvalue (Game|SpawnActorfromClass "/Game/Blueprints/Characters/BP_GrapplePoint.BP_GrapplePoint_C" (Math|Transform|MakeTransform (Transformation|GetSocketLocation (Variables|/Script/Engine.Character|GetMesh _output_get) "spine_05")) "Undefined" "MultiplyWithRoot" 0 0))
  (bind _output_get_2 (Variables|Default|SetGrapplePoint _returnvalue))
  (Rendering|SetVisibility (Variables|Default|GetCable) true false)
  (Variables|Default|SetIsGrappling true)
  (Transformation|AttachActorToActor _output_get_2 (Variables|Default|GetCharacterPossessing) "None" "KeepWorld" "KeepWorld" "KeepWorld" true)
  (bind _asgameplay_pc (Utilities|Casting|CastToGameplayPC (Game|GetPlayerController 0)))
  (Class|GameplayPC|SetCameraRotationEnabled _asgameplay_pc false))

(event Custom|StartGrapple
  ;[1 1 1] StartGrapple
  (if (Variables|Default|GetCanGrapple)
    (bind (_hitres _ifhit) (CallFunction|RayCastforGrapple))
    (Variables|Default|SetHasHit _ifhit)
    (Variables|Default|SetDist (.Distance (Collision|BreakHitResult _hitres)))
    (Variables|Default|SetGrappleStart (.TraceStart (Collision|BreakHitResult _hitres)))
    (if (Variables|Default|GetHasHit)
      (bind _returnvalue (Game|SpawnActorfromClass "/Game/Blueprints/Characters/BP_GrapplePoint.BP_GrapplePoint_C" (Math|Transform|MakeTransform (.ImpactPoint (Collision|BreakHitResult _hitres))) "Undefined" "MultiplyWithRoot" 0 0))
      (bind _output_get (Variables|Default|SetGrapplePoint _returnvalue))
      (else
        (bind _returnvalue_2 (Game|SpawnActorfromClass "/Game/Blueprints/Characters/BP_GrapplePoint.BP_GrapplePoint_C" (Math|Transform|MakeTransform (.TraceEnd (Collision|BreakHitResult _hitres))) "Undefined" "MultiplyWithRoot" 0 0))
        (Variables|Default|SetGrapplePoint _returnvalue_2)))
    (Rendering|SetVisibility (Variables|Default|GetCable) true false)
    (Variables|Default|SetIsGrappling true)
    (if (Variables|Default|GetHasHit)
      (Transformation|AttachActorToActor _output_get (.HitActor (Collision|BreakHitResult _hitres)) "None" "KeepWorld" "KeepWorld" "KeepWorld" true)
      (Pawn|Components|CharacterMovement|SetMovementMode (Variables|/Script/Engine.Character|GetCharacterMovement (Variables|Default|GetParentCharacter)) "MOVE_Flying" 0)
      (Utilities|Time|SetTimerbyEvent (delegate Custom|PlayTimerSound) 0.25 (and (Variables|Default|GetIsGrappling) (Variables|Default|GetHasHit)) (/ (Variables|Default|GetGrappleDurationTime) 2.0)))))

(event Custom|GrapplePlayer
  (params (DeltaSec :type Float%20%28double-precision%29))
  ;[1 1 1] GrapplePlayer
  (if (Variables|Default|GetIsGrappling)
    (Variables|Default|SetGrappleCurrentTime (+ DeltaSec (Variables|Default|GetGrappleCurrentTime)))
    (if (< (+ DeltaSec (Variables|Default|GetGrappleCurrentTime)) (Variables|Default|GetGrappleDurationTime))
      (CallFunction|DrawGrapple)
      (if (Variables|Default|GetHasHit)
        (CallFunction|GrappleMovement))
      (else
        (CallFunction|StopGrapple)))))

(event Custom|SetPossessCooldown
  (params (CanPossess :type Boolean) (PossessCooldown :type Float%20%28double-precision%29))
  ;[1 1 1] Possesion
  (Variables|Default|SetCanPossess CanPossess)
  (Variables|Default|SetHighlightedCharacter 0)
  (Utilities|FlowControl|Delay PossessCooldown)
  (Variables|Default|SetCanPossess true))

(event EventBeginPlay
  (bind _asbp_base_character (Utilities|Casting|CastToBP_BaseCharacter (Components|GetOwner)))
  (bind _output_get (Variables|Default|SetParentCharacter _asbp_base_character))
  (Variables|Default|SetCable (Variables|/Game/Blueprints/Characters/BP_BaseCharacter.BP_BaseCharacter_C|GetCable _output_get)))

(event EventTick
  (params (DeltaSeconds :type Float%20%28single-precision%29))
  (CallFunction|GrapplePlayer DeltaSeconds)
  (CallFunction|HighlightPossess)
  (CallFunction|UpdatePossess DeltaSeconds))

(event Input|MouseEvents|RightMouseButton
  (params (Key :type Key%20Structure :default "None"))
  (bind _ispossessing (Variables|Default|GetIsPossessing))
  ;[1 1 1] Input
  (:Pressed
    (if (not _ispossessing)
      (bind (_hitres _ifhit) (CallFunction|RayCastforPossession))
      (if _ifhit
        (CallFunction|Possess (.HitActor (Collision|BreakHitResult _hitres)))
        (else
          (CallFunction|StartGrapple)))))
  (:Released
    (if (not _ispossessing)
      (CallFunction|StopGrapple))))

(fn RayCastforGrapple
  ;[1 1 1] RayCast
  (bind _asbase_character (Utilities|Casting|CastToBaseCharacter (Components|GetOwner)))
  (bind _outactors (Actor|GetAllActorsOfClass (Utilities|GetClass (Components|GetOwner))))
  (bind (_outhit _returnvalue) (Collision|LineTraceByChannel (Transformation|GetWorldLocation (Class|BaseCharacter|GetFirstPersonCamera _asbase_character)) (+ (Transformation|GetWorldLocation (Class|BaseCharacter|GetFirstPersonCamera _asbase_character)) (* (Math|Vector|GetForwardVector (Class|BaseCharacter|GetFirstPersonCamera _asbase_character)) (Variables|Default|GetGrappleLength))) "TraceTypeQuery1" false _outactors "None"))
  (return _outhit _returnvalue))

(fn RayCastforPossession
  ;[1 1 1] RayCast
  (bind _asbase_character (Utilities|Casting|CastToBaseCharacter (Components|GetOwner)))
  (bind (_outhit _returnvalue) (Collision|LineTraceByChannel (Transformation|GetWorldLocation (Class|BaseCharacter|GetFirstPersonCamera _asbase_character)) (+ (Transformation|GetWorldLocation (Class|BaseCharacter|GetFirstPersonCamera _asbase_character)) (* (Math|Vector|GetForwardVector (Class|BaseCharacter|GetFirstPersonCamera _asbase_character)) (Variables|Default|GetGrappleLength))) "TraceTypeQuery1" false 0 "None"))
  (if _returnvalue
    (bind _asbase_character_2 (Utilities|Casting|CastToBaseCharacter (.HitActor (Collision|BreakHitResult _outhit)))
      (:then
        (return _outhit (and _returnvalue (CallFunction|CanPossessOther _asbase_character_2))))
      (:CastFailed
        _)))
  (bind (_outhit_2 _returnvalue_2) (Collision|SphereTraceByChannel (Transformation|GetWorldLocation (Class|BaseCharacter|GetFirstPersonCamera _asbase_character)) (+ (Transformation|GetWorldLocation (Class|BaseCharacter|GetFirstPersonCamera _asbase_character)) (* (Math|Vector|GetForwardVector (Class|BaseCharacter|GetFirstPersonCamera _asbase_character)) (Variables|Default|GetGrappleLength))) 5e+01 "TraceTypeQuery1" false 0 "None"))
  (bind _asbase_character_3 (Utilities|Casting|CastToBaseCharacter (.HitActor (Collision|BreakHitResult _outhit_2)))
    (:then
      (return _outhit_2 (and _returnvalue_2 (CallFunction|CanPossessOther _asbase_character_3))))
    (:CastFailed
      (return _outhit_2 false))))

(fn CanPossessOther
  (params (CharacterToCheck :type Base%20Character%20Object%20Reference))
  (return true))