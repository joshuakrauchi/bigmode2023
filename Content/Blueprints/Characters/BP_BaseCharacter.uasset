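; Base character Blueprint for possessable, colour-coded characters, handling audio, animation and UI feedback for player and AI control.
; On possession it toggles first-person mesh animation and, for players, matches the cable material and plays colour-mode sounds, skipped at certain combo counts.
; A looping timer scales wind volume with player speed.
; Other events cover damage feedback, pausing, and starting a collision-free move to a safe spawner, the latter two stopping the grapple.
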(event Custom|StartMove
  (params (Location :type Vector))
  (Default|StopGrapple (Variables|Default|GetBP_GrappleComponent))
  (Variables|Default|SetSafeSpawnerLocation Location)
  (Variables|Default|SetbIsMovingToSafeSpawner true)
  (Input|SetIgnoreMoveInput (Pawn|GetController) true)
  (Collision|SetCollisionEnabled (Variables|Default|GetCapsuleComponent) "NoCollision"))

(event Custom|WindVolume
  (if (Pawn|IsPlayerControlled)
    (Audio|Components|Audio|AdjustVolume (Variables|Default|GetWind) 0.25 (Math|Float|Clamp(Float) (/ (Math|Vector|VectorLength (Transformation|GetVelocity)) 2e+03) 0.5 1.25) "Linear" :!class /Script/Engine.AudioComponent)))

(event Input|EnhancedActionEvents|EnhancedInputActionIA_Pause
  (params (ActionValue :type Boolean) (ElapsedSeconds :type Float%20%28double-precision%29) (TriggeredSeconds :type Float%20%28double-precision%29) (InputAction :type Input%20Action%20Object%20Reference :default "/Game/Input/InputActions/IA_Pause.IA_Pause"))
  (if (not (Game|IsGamePaused))
    (bind _returnvalue (UserInterface|CreateWidget "/Game/Blueprints/UI/BP_MainMenu.BP_MainMenu_C"))
    (bind _output_get (Variables|Default|SetMainMenu _returnvalue))
    (UserInterface|Viewport|AddtoViewport _output_get 10)
    (Game|SetGamePaused true)
    (Default|StopGrapple (Variables|Default|GetBP_GrappleComponent))))

(event EventPlayDamagedMontage
  (Variables|Default|SetbIsPlayingDamagedMontage true)
  (Animation|Montage|PlayMontage (Variables|Character|GetMesh) "/Game/Assets/Animations/AM_DamageReaction.AM_DamageReaction"
    (:OnCompleted
      (Variables|Default|SetbIsPlayingDamagedMontage false))))

(event EventPossessed
  (params (NewController :type Controller%20Object%20Reference))
  (bind _returnvalue (Pawn|IsPlayerControlled))
  (bind _firstpersonmesh (Variables|Default|GetFirstPersonMesh))
  (Components|Tick|SetComponentTickEnabled _firstpersonmesh _returnvalue)
  (if _returnvalue
    (Class|SkeletalMeshComponent|SetAnimClass _firstpersonmesh "/Game/Blueprints/Characters/ABP_Player.ABP_Player_C")
    (Rendering|Material|SetMaterial (Variables|Default|GetCable) 0 (Rendering|Material|GetMaterial (Variables|Character|GetMesh) 0))
    (Audio|PlaySound2D "/Game/Assets/Audio/Character/Possesion.Possesion" 1.0 1.0 0.0 0 0)
    (Audio|PlaySound2D "/Game/Assets/Audio/Character/possesssfx.possesssfx" 1.0 1.0 0.0 0 0)
    (bind _asbp_gameplay_gs (Utilities|Casting|CastToBP_GameplayGS (Game|GetGameState)))
    (if (not (== (Math|Integer|%(Integer) (Variables|/Script/ModeGame.GameplayGS|GetCurrentComboCount _asbp_gameplay_gs) 10) 9))
      (switch Utilities|FlowControl|Switch|SwitchonEPlayableColours (Variables|Default|GetCharacterColour)
        (:Red
          (Audio|PlaySound2D "/Game/Assets/Audio/Character/redmode.redmode" 1.0 1.0 0.0 0 0))
        (:Green
          (Audio|PlaySound2D "/Game/Assets/Audio/Character/greenmode.greenmode" 1.0 1.0 0.0 0 0))
        (:Blue
          (Audio|PlaySound2D "/Game/Assets/Audio/Character/bluemode.bluemode" 1.0 1.0 0.0 0 0))))
    (else
      (Class|SkeletalMeshComponent|SetAnimClass _firstpersonmesh))))

(event EventBeginPlay
  (bind _wind (Variables|Default|GetWind))
  (Audio|Components|Audio|Stop _wind)
  (Audio|Components|Audio|FadeIn _wind 0.0 0.0 0.0 "Linear" :!class /Script/Engine.AudioComponent)
  (Utilities|Time|SetTimerbyEvent (delegate Custom|WindVolume) 0.25 true))

(event EventPlayDamagedAISFX
  (Audio|PlaySound2D "/Game/Assets/Audio/Character/hitmarkersfx.hitmarkersfx" 1.0 1.0 0.0 0 0))

(event EventPlayDamagedPlayerSFX
  (Audio|PlaySound2D "/Game/Assets/Audio/Character/damaged.damaged" 1.0 1.0 0.0 0 0))

(event EventPlayDoubleJumpSFX
  (Audio|PlaySoundatLocation "/Game/Assets/Audio/Character/jump.jump" "0, 0, 0" "0, 0, 0" 1.0 1.0 0.0 "/Game/Assets/Audio/WorldSoundAttenuation.WorldSoundAttenuation" 0 0 0))

(event EventCreateDamageIndicator
  (params (DamageStartLocation :type Vector :default "0, 0, 0") (DamageColor :type Linear%20Color%20Structure))
  (bind _returnvalue (UserInterface|CreateWidget "/Game/Blueprints/UI/BP_DamageIndicator.BP_DamageIndicator_C"))
  (Variables|/Game/Blueprints/UI/BP_DamageIndicator.BP_DamageIndicator_C|SetPlayerCharacter _returnvalue self)
  (Variables|/Game/Blueprints/UI/BP_DamageIndicator.BP_DamageIndicator_C|SetDamageStartLocation _returnvalue DamageStartLocation)
  (Variables|/Game/Blueprints/UI/BP_DamageIndicator.BP_DamageIndicator_C|SetDamageColor _returnvalue DamageColor)
  (UserInterface|Viewport|AddtoViewport _returnvalue 0))

(event EventOnJumped
  (Audio|PlaySoundatLocation "/Game/Assets/Audio/Character/jump.jump" "0, 0, 0" "0, 0, 0" 1.0 1.0 0.0 "/Game/Assets/Audio/WorldSoundAttenuation.WorldSoundAttenuation" 0 0 0))

(fn ConstructionScript)