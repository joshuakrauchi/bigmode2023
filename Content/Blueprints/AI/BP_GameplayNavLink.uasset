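; BP_GameplayNavLink is a smart nav link that makes AI characters jump to the link's destination.
; When an agent reaches the link, it casts to BaseCharacter and launches it, overriding existing XY and Z velocity.
; CalculateVelocity solves a ballistic arc from agent to destination, with flight time scaled by distance at a fixed speed and a hard-coded gravity term.
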(event EventBeginPlay)

(event Collision|EventActorBeginOverlap
  (params (OtherActor :type Actor%20Object%20Reference)))

(event EventTick
  (params (DeltaSeconds :type Float%20%28single-precision%29)))

(event EventSmartLinkReached
  (params (Agent :type Actor%20Object%20Reference) (Destination :type Vector%20%28by%20ref%29 :default "0, 0, 0"))
  (bind _returnvalue (Transformation|GetActorLocation Agent))
  (bind _asbase_character (Utilities|Casting|CastToBaseCharacter Agent))
  (Character|LaunchCharacter _asbase_character (CallFunction|CalculateVelocity _returnvalue Destination (/ (Math|Vector|Distance(Vector) Destination _returnvalue) 4e+02)) true true))

(fn ConstructionScript)

(fn CalculateVelocity
  (params (Start :type Vector) (Target :type Vector) (Duration :type Float%20%28double-precision%29))
  (return (Math|Vector|MakeVector (/ (- (.x Target) (.x Start)) Duration) (/ (- (.y Target) (.y Start)) Duration) (/ (- (.z Target) (+ (.z Start) (* (Math|Float|Square Duration) -491.0))) Duration))))