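; BP_GreyWeapon is a hitscan weapon that plays pistol firing animations on its owning character's first-person and body meshes.
; ReceiveTestFire sphere-traces along the Visibility channel to max range with no scatter, then spawns a Niagara trail from the muzzle to the impact or end point.
; Damageable hits go through TryDamageDamageable with hit distance, while other blocking hits leave an attached decal.
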(event Custom|PlayFiringMontage
  (bind _asbase_character (Utilities|Casting|CastToBaseCharacter (Components|GetOwner)))
  (Animation|Montage|PlayMontage (Class|BaseCharacter|GetFirstPersonMesh _asbase_character) "/Game/Assets/Animations/AM_FirePistol.AM_FirePistol"
    (:then
      (Animation|Montage|PlayMontage (Variables|/Script/Engine.Character|GetMesh _asbase_character) "/Game/Assets/Animations/AM_FirePistol.AM_FirePistol"))))

(event Custom|SpawnDecal
  (params (Location :type Vector) (Normal :type Vector) (Attach%20Component :type Scene%20Component%20Object%20Reference))
  (bind _returnvalue (Class|GameplayStatics|SpawnDecalAttached 0 (Math|Conversions|ToVector(Float) (Variables|Default|GetDecalSize)) Attach%20Component "None" Location (Math|Conversions|RotationFromXVector Normal) "KeepWorldPosition" 3e+02))
  (Rendering|Components|Decal|SetFadeScreenSize _returnvalue 0.0))

(event Custom|SpawnBulletTrail
  (params (Beam%20End :type Vector))
  (bind _returnvalue (Niagara|SpawnSystematLocation "/Game/Assets/Particles/NS_GreyBulletTrail.NS_GreyBulletTrail" (Transformation|GetSocketLocation (Class|BaseWeapon|GetVisibleMesh) "Muzzle")))
  (Niagara|SetNiagaraVariable(Vector3) _returnvalue "Beam End" Beam%20End))

(event EventBeginPlay)

(event Collision|EventActorBeginOverlap
  (params (OtherActor :type Actor%20Object%20Reference)))

(event EventTick
  (params (DeltaSeconds :type Float%20%28single-precision%29)))

(fn ConstructionScript)

(fn ReceiveTestFire
  (bind _asbase_character (Utilities|Casting|CastToBaseCharacter (Components|GetOwner)))
  (CallFunction|PlayFiringMontage)
  (bind _output_get (LocalVariables|SetCurrentProjectileEndLocation (Class|BaseCharacter|GetProjectileEndLocation _asbase_character (Variables|Default|GetMaxRange) 0.0)))
  (bind _outhit (Collision|SphereTraceByChannel (Class|BaseCharacter|GetProjectileStartLocation _asbase_character) _output_get 3e+01 "TraceTypeQuery1" false (Utilities|Array|MakeArray _asbase_character) "None" true "(R=1.000000,G=0.000000,B=0.000000,A=1.000000)" "(R=0.000000,G=1.000000,B=0.000000,A=1.000000)" 1.0))
  (if (.bblockinghit _outhit)
    (CallFunction|SpawnBulletTrail (.impactpoint _outhit))
    (bind _asdamageable (Utilities|Casting|CastToDamageable (.hitactor _outhit))
      (:then
        (bind _returnvalue (Class|BaseWeapon|TryDamageDamageable _asdamageable (.distance _outhit)))
        (return _returnvalue))
      (:CastFailed
        (CallFunction|SpawnDecal (.impactpoint _outhit) (.impactnormal _outhit) (.hitcomponent _outhit))))
    (else
      (CallFunction|SpawnBulletTrail (LocalVariables|GetCurrentProjectileEndLocation)))))