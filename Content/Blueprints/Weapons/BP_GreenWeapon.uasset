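; Green weapon Blueprint that supplies shotgun firing animation and sound.
; PlayFiringMontage plays the shotgun montage on the owning BaseCharacter's mesh, and also on the first-person mesh when player-controlled.
; PlayFiringSFX plays the firing sound, as does ReceiveTestFire, which then returns true.
; A disconnected test in ReceiveTestFire, which never runs, traces eight randomly spread debug rays from the equipped transform.
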(event EventBeginPlay)

(event Collision|EventActorBeginOverlap
  (params (OtherActor :type Actor%20Object%20Reference)))

(event EventTick
  (params (DeltaSeconds :type Float%20%28single-precision%29)))

(event EventPlayFiringMontage
  (bind _asbase_character (Utilities|Casting|CastToBaseCharacter (Components|GetOwner)))
  (Animation|Montage|PlayMontage (Variables|/Script/Engine.Character|GetMesh _asbase_character) "/Game/Assets/Animations/AM_FireShotgun.AM_FireShotgun"
    (:then
      (if (Pawn|IsPlayerControlled _asbase_character)
        (Animation|Montage|PlayMontage (Class|BaseCharacter|GetFirstPersonMesh _asbase_character) "/Game/Assets/Animations/AM_FireShotgun.AM_FireShotgun")))))

(event EventPlayFiringSFX
  (Audio|Components|Audio|Play (Variables|Default|GetFiringSFX) 0.0))

(fn ConstructionScript)

(fn ReceiveTestFire
  (Audio|Components|Audio|Play (Variables|Default|GetFiringSFX) 0.0)
  (return true))